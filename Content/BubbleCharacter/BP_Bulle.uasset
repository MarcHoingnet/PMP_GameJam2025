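; Player bubble character that moves along world X through Enhanced Input and plays a start sound on BeginPlay.
; Each tick pins the spring arm to fixed X/Y so the camera follows only the bubble's height.
; Tick also overrides vertical velocity using Vitesse as a clamp floor and points gravity along the velocity.
; A capsule physics velocity write on Tick is marked as uncertain to work.
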(event `self.ReceiveBeginPlay`
  (bind _asplayer_controller (cast `PlayerController` (`self.GetController`)))
  (`EnhancedInputSubsystemInterface.AddMappingContext` (pcsubsystem `EnhancedInputLocalPlayerSubsystem` _asplayer_controller) "/Game/BubbleCharacter/Input/IMC_Bubble.IMC_Bubble" 0 (struct))
  (`GameplayStatics.PlaySound2D` "/Game/SoundDesign/SFX/2DSounds/Start2D.Start2D" 1.0 1.0 0.0 null null))

(event `self.ReceiveTick`
  (params (DeltaSeconds :type "Float (single-precision)"))
  (bind (_returnvalue_x _returnvalue_y _returnvalue_z) (`KismetMathLibrary.BreakVector` (`self.K2_GetActorLocation`)))
  (bind _charactermovement (`self.CharacterMovement`))
  (bind (_velocity_x _velocity_y) (`KismetMathLibrary.BreakVector` (`MovementComponent.Velocity` _charactermovement)))
  (`SceneComponent.K2_SetWorldLocation` (`self.SpringArm`) (`KismetMathLibrary.MakeVector` 2120.0 1070.0 _returnvalue_z) false false)
  (bind _output_get (set `MovementComponent.Velocity` (`KismetMathLibrary.MakeVector` _velocity_x _velocity_y (`KismetMathLibrary.FClamp` 0.0 (`self.Vitesse`) 400.0)) _charactermovement))
  (`CharacterMovementComponent.SetGravityDirection` (`self.CharacterMovement`) _output_get)
  ; jsp si ca marche
  (`PrimitiveComponent.SetPhysicsLinearVelocity` (`self.CapsuleComponent`) (0.0 0.0 1.0) false "None"))

(event `EnhancedInput|/Game/BubbleCharacter/Input/Actions/IA_BubbleMovement`
  (params (ActionValue :type "Float (double-precision)") (ElapsedSeconds :type "Float (double-precision)") (TriggeredSeconds :type "Float (double-precision)") (InputAction :type "InputAction Object Reference" :default "/Game/BubbleCharacter/Input/Actions/IA_BubbleMovement.IA_BubbleMovement"))
  (:`Triggered`
    (`self.AddMovementInput` (1.0 0.0 0.0) ActionValue)))

(fn `UserConstructionScript`)