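; Playable ladybug (coccinelle) 2D flipbook character that runs and jumps via Enhanced Input, with sound effects and a health widget.
; Movement input and velocity drive flipbook changes, and Tick flips control yaw to face the travel direction.
; Any damage removes one health point.
; At zero, Tick triggers a DoOnce-guarded HealFull that plays death, disables input and collision, then after a delay restarts the level and resets state.
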(event `self.ReceiveAnyDamage`
  (params (Damage :type "Float (single-precision)") (DamageType :type "DamageType Object Reference") (InstigatedBy :type "Controller Object Reference") (DamageCauser :type "Actor Object Reference"))
  (bind _currenthealth (`self.CurrentHealth`))
  ; dégat
  (set `self.CurrentHealth` (`KismetMathLibrary.Max` 0 (- _currenthealth 1)))
  (`GameplayStatics.PlaySound2D` "/Game/SoundDesign/SFX/2DSounds/Hit2D.Hit2D" 1.0 1.0 0.0 null null)
  (`/Game/2Dcharacter/Widgets/WB_Gameplay.Set Health` (`self.W_Gameplay`) _currenthealth (`self.MaxHealth`)))

(event `HealFull`
  (bind _currenthealth (`self.CurrentHealth`))
  (bind _maxhealth (`self.MaxHealth`))
  (`/Engine/EditorBlueprintResources/StandardMacros.DoOnce` false :!label _label
    (:`Completed`
      (`GameplayStatics.PlaySound2D` "/Game/SoundDesign/SFX/2DSounds/Mort2D.Mort2D" 1.0 1.0 0.0 null null)
      (`self.SetActorEnableCollision` false)
      (set `self.Isdead` true)
      (`PaperFlipbookComponent.SetFlipbook` (`self.Sprite`) "/Game/2Dcharacter/Coccinelle/CoccinelleDeath_Flipbook.CoccinelleDeath_Flipbook")
      (`self.DisableInput` self null)
      ; Soin surtout utilisé apres une mort
      (`KismetSystemLibrary.Delay` 2.0)
      (`KismetSystemLibrary.ExecuteConsoleCommand` "RestartLevel" null)
      (set `self.CurrentHealth` (`KismetMathLibrary.Min` (`self.MaxHealth`) (+ _maxhealth _currenthealth)))
      (`/Game/2Dcharacter/Widgets/WB_Gameplay.Set Health` (`self.W_Gameplay`) _currenthealth _maxhealth)
      (`self.EnableInput` null)
      (set `self.Isdead` false)
      (`self.SetActorEnableCollision` true)
      (goto _label :!via `Reset`))))

(event `self.ReceiveBeginPlay`
  (`GameplayStatics.PlaySound2D` "/Game/SoundDesign/SFX/2DSounds/Start2D.Start2D" 1.0 1.0 0.0 null null)
  (`|ExecutionSequence`
    (:`then_0`
      (bind _returnvalue (`|CreateWidget` "/Game/2Dcharacter/Widgets/WB_Gameplay.WB_Gameplay_C"))
      (bind _output_get (set `self.W_Gameplay` _returnvalue))
      (`UserWidget.AddToViewport` _output_get 0)
      (set `self.MaxHealth` (`self.MaxHealth`)))
    (:`then_1`
      (bind _asplayer_controller (cast `PlayerController` (`self.GetController`)))
      (`EnhancedInputSubsystemInterface.AddMappingContext` (pcsubsystem `EnhancedInputLocalPlayerSubsystem` _asplayer_controller) "/Game/2Dcharacter/Input/IMC_2D.IMC_2D" 0 (struct))
      (set `self.CurrentHealth` (`self.MaxHealth`)))))

(event `self.ReceiveTick`
  (params (DeltaSeconds :type "Float (single-precision)"))
  (bind _returnvalue_x (`KismetMathLibrary.BreakVector` (`self.GetVelocity`)))
  (if (== (`self.CurrentHealth`) 0)
    (`self.HealFull`)
    (else
      (`self.SetCharRotation`)
      (if (== _returnvalue_x 0.0)
        (if (`NavMovementComponent.IsFalling` (`self.CharacterMovement`))
          _
          (elif (not (`self.Isdead`))
            (`PaperFlipbookComponent.SetFlipbook` (`self.Sprite`) "/Game/2Dcharacter/Coccinelle/CoccinelleIdle_Flipbook.CoccinelleIdle_Flipbook")))))))

(event `EnhancedInput|/Game/2Dcharacter/Input/Actions/IA_Move2D`
  (params (ActionValue :type "Float (double-precision)") (ElapsedSeconds :type "Float (double-precision)") (TriggeredSeconds :type "Float (double-precision)") (InputAction :type "InputAction Object Reference" :default "/Game/2Dcharacter/Input/Actions/IA_Move2D.IA_Move2D"))
  (:`Triggered`
    (`self.AddMovementInput` (1.0 0.0 0.0) ActionValue)
    (if (`NavMovementComponent.IsFalling` (`self.CharacterMovement`))
      (`PaperFlipbookComponent.SetFlipbook` (`self.Sprite`) "/Game/2Dcharacter/Coccinelle/CoccinelleJump_Flipbook.CoccinelleJump_Flipbook")
      (else
        (`PaperFlipbookComponent.SetFlipbook` (`self.Sprite`) "/Game/2Dcharacter/Coccinelle/CoccinelleRun.CoccinelleRun")))))

(event `EnhancedInput|/Game/2Dcharacter/Input/Actions/IA_Jump2D`
  (params (ActionValue :type Boolean) (ElapsedSeconds :type "Float (double-precision)") (TriggeredSeconds :type "Float (double-precision)") (InputAction :type "InputAction Object Reference" :default "/Game/2Dcharacter/Input/Actions/IA_Jump2D.IA_Jump2D"))
  (:`Started`
    (`self.Jump`)
    (`PaperFlipbookComponent.SetFlipbook` (`self.Sprite`) "/Game/2Dcharacter/Coccinelle/CoccinelleJump_Flipbook.CoccinelleJump_Flipbook")
    (`GameplayStatics.PlaySound2D` "/Game/SoundDesign/SFX/2DSounds/Jump2D.Jump2D" 1.0 1.0 0.0 null null))
  (:`Completed`
    (`self.StopJumping`)))

(event `SetCharRotation`
  (bind _returnvalue (`self.GetController`))
  (bind _returnvalue_2 (`self.GetController`))
  (`/Engine/EditorBlueprintResources/StandardMacros.CompareFloat` (.x (`MovementComponent.Velocity` (`self.GetMovementComponent`)))
    (:`>`
      ;[1 1 1] droite
      (`/Engine/EditorBlueprintResources/StandardMacros.IsValid` _returnvalue_2
        (:`Is Valid`
          (`Controller.SetControlRotation` _returnvalue_2 (`KismetMathLibrary.MakeRotator` 0.0)))))
    (:`<`
      ;[1 1 1] gauche
      (`/Engine/EditorBlueprintResources/StandardMacros.IsValid` _returnvalue
        (:`Is Valid`
          (`Controller.SetControlRotation` _returnvalue (`KismetMathLibrary.MakeRotator` 0.0 0.0 180.0)))))))

(fn `UserConstructionScript`)