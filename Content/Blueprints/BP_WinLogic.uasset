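; BP_WinLogic is an actor that ends the game once all win conditions are met.
; Every tick it checks the MarmotteWon, Tournesol and BubbleWon flags on the GI_Game game instance.
; When all three are true, it runs once: after a delay it shows the WB_Fin end widget, then after another delay opens the MapMenuRoom level.
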(event `self.ReceiveTick`
  (params (DeltaSeconds :type "Float (single-precision)"))
  (bind _asgi_game (cast `/Game/Blueprints/GI_Game` (`GameplayStatics.GetGameInstance`)))
  (if (`/Game/Blueprints/GI_Game.MarmotteWon` _asgi_game)
    (if (`/Game/Blueprints/GI_Game.Tournesol` _asgi_game)
      (if (`/Game/Blueprints/GI_Game.BubbleWon` _asgi_game)
        (`/Engine/EditorBlueprintResources/StandardMacros.DoOnce` false
          (:`Completed`
            (`KismetSystemLibrary.Delay` 7.0)
            (bind _returnvalue (`|CreateWidget` "/Game/Blueprints/Widgets/FINS/WB_Fin.WB_Fin_C"))
            (`UserWidget.AddToViewport` _returnvalue 0)
            (`KismetSystemLibrary.Delay` 8.0)
            (`GameplayStatics.OpenLevelBySoftObjectPtr` "/Game/FirstPerson/Maps/MapMenuRoom.MapMenuRoom")))))))

(fn `UserConstructionScript`)