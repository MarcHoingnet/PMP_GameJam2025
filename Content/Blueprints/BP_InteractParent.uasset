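; BP_InteractParent is a base interactable actor that signals when something enters its Box trigger.
; Overlap begin sets IsInteract, adds a new WB_Interact widget to the viewport and enables custom depth with a stencil value on Cube0 for highlighting.
; Overlap end reverses the flag, widget and custom depth, without filtering the overlapping actor.
; The IA_Interact input does nothing yet, and Interact only enables custom depth.
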(event `EnhancedInput|/Game/FirstPerson/Input/Actions/IA_Interact`
  (params (ActionValue :type Boolean) (ElapsedSeconds :type "Float (double-precision)") (TriggeredSeconds :type "Float (double-precision)") (InputAction :type "InputAction Object Reference" :default "/Game/FirstPerson/Input/Actions/IA_Interact.IA_Interact"))
  (:`Triggered`
    (if true
      _)))

(event `self.Box.OnComponentBeginOverlap`
  (params (OverlappedComponent :type "PrimitiveComponent Object Reference") (OtherActor :type "Actor Object Reference") (OtherComp :type "PrimitiveComponent Object Reference") (OtherBodyIndex :type Integer) (bFromSweep :type Boolean) (SweepResult :type "HitResult Structure (by ref)"))
  (set `self.IsInteract` true)
  (bind _returnvalue (`|CreateWidget` "/Game/Blueprints/Widgets/WB_Interact.WB_Interact_C"))
  (bind _output_get (set `self.RefWidgetInteract` _returnvalue))
  (`UserWidget.AddToViewport` _output_get 0)
  (`PrimitiveComponent.SetRenderCustomDepth` (`self.cube_0`) true)
  (`PrimitiveComponent.SetCustomDepthStencilValue` (`self.cube_0`) 5))

(event `self.Box.OnComponentEndOverlap`
  (params (OverlappedComponent :type "PrimitiveComponent Object Reference") (OtherActor :type "Actor Object Reference") (OtherComp :type "PrimitiveComponent Object Reference") (OtherBodyIndex :type Integer))
  (set `self.IsInteract` false)
  (`Widget.RemoveFromParent` (stale `self.Box.OnComponentBeginOverlap` _returnvalue))
  (`PrimitiveComponent.SetRenderCustomDepth` (`self.cube_0`) false))

(fn `Interact`
  (`PrimitiveComponent.SetRenderCustomDepth` (`self.cube_0`) true))

(fn `UserConstructionScript`)